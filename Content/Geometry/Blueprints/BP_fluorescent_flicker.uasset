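; Fluorescent tube fixture that flickers by driving a rect light and the tube's emissive material together.
; Each Tick, time-scaled Perlin noise is remapped to a wide range and clamped, then scales light intensity and emissive color, with a small minimum glow on the material.
; The construction script previews light color, intensity and emissive tint in-editor through a dynamic material instance, which BeginPlay recreates.
; The per-frame update is flagged as costly.
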(event `self.ReceiveBeginPlay`
  ;[0.1 0.1 0.1] Create Dyn Mat Instance
  (bind _returnvalue (`KismetMaterialLibrary.CreateDynamicMaterialInstance` "/Game/Materials/Props/MI_fluorescent_tube.MI_fluorescent_tube" "FlickerMat"))
  (bind _output_get (set `self.flickerMat` _returnvalue))
  (`PrimitiveComponent.SetMaterial` (`self.SM_fluorescent_1`) 1 _output_get))

(event `self.ReceiveTick`
  (params (DeltaSeconds :type "Float (single-precision)"))
  (bind _returnvalue (`KismetMathLibrary.FClamp` (`KismetAnimationLibrary.K2_MakePerlinNoiseAndRemap` (* (`GameplayStatics.GetTimeSeconds`) (`self.Flicker Speed`)) -2.0 5.0)))
  ;[0.1 0.1 0.1] Update Intensity (light and material)
  (`MaterialInstanceDynamic.SetVectorParameterValue` (`self.flickerMat`) "Emissive Color" (* (`self.Light Color`) (+ (* _returnvalue (`self.Fluorescent Buld Intensity`)) 0.1)))
  (`LightComponent.SetIntensity` (`self.RectLight`) (* _returnvalue (`self.Light Intensity`))))

(fn `UserConstructionScript`
  (bind _rectlight (`self.RectLight`))
  ;[0.1 0.1 0.1] Make it so that in-editor we can see the Light Intensity change
  (`LightComponent.SetIntensity` _rectlight (`self.Light Intensity`))
  (`LightComponent.SetLightColor` _rectlight (`self.Light Color`) true)
  ;[0.1 0.1 0.1] Create Dyn Mat Instance (for In-Editor Visualisation)
  (bind _returnvalue (`KismetMaterialLibrary.CreateDynamicMaterialInstance` "/Game/Materials/Props/MI_fluorescent_tube.MI_fluorescent_tube" "FlickerMat"))
  (bind _output_get (set `self.flickerMat` _returnvalue))
  (`MaterialInstanceDynamic.SetVectorParameterValue` _output_get "Emissive Color" (`self.Light Color`))
  (`PrimitiveComponent.SetMaterial` (`self.SM_fluorescent_1`) 1 _output_get))